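; BP_SlidingDoor is a keyed door that slides upward when interacted with and the game mode's key value matches its KeyNumber.
; It caches BP_ThirdPersonGameMode on BeginPlay and compares Keys for exact equality on Interact.
; A match plays a timeline that lerps the Door's relative location, with no closing logic; a mismatch prints a message.
; The Construction Script applies a configurable material to the Door.
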(event Collision|EventActorBeginOverlap
  (params (OtherActor :type Actor%20Object%20Reference)))

(event EventBeginPlay
  (bind _asbp_third_person_game_mode (Utilities|Casting|CastToBP_ThirdPersonGameMode (Game|GetGameMode)))
  (Variables|Default|SetAs%20BP%20Third%20Person%20Game%20Mode _asbp_third_person_game_mode))

(event EventInteract
  (if (== (Variables|/Game/ThirdPerson/Blueprints/BP_ThirdPersonGameMode.BP_ThirdPersonGameMode_C|GetKeys (Variables|Default|GetAs%20BP%20Third%20Person%20Game%20Mode)) (Variables|Default|GetKeyNumber))
    (bind _newtrack_0 (Timeline|Timeline Play)
      (:Update
        (Transformation|SetRelativeLocation (Variables|Default|GetDoor) (Math|Vector|Lerp(Vector) "0, 0, 0" "0.000000,0.000000,300.000000" _newtrack_0) false false)))
    (else
      (Development|PrintString "You Dont have to correct key"))))

(fn ConstructionScript
  (Rendering|Material|SetMaterial (Variables|Default|GetDoor) 0 (Variables|Default|GetMaterial)))